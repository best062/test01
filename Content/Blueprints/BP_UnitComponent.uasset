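; Unit component that handles basic combat: attacking, taking damage and death.
; Attack, while alive, calls ReceiveDamage on the target with ATK minus the target's DEF, floored at one.
; ReceiveDamage, while alive, sets HP to incoming damage minus current HP (not HP minus damage), clamped between zero and MaxHP.
; At zero HP it clears IsAlive and prints a death message.
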(event Custom|ReceiveDamage
  (params (Damage :type Float%20%28double-precision%29))
  (if (Variables|Default|GetIsAlive)
    (bind _output_get (Variables|Default|SetHP (Math|Float|Clamp(Float) (- Damage (Variables|Default|GetHP)) 0.0 (Variables|Default|GetMaxHP))))
    (if (<= _output_get 0.0)
      (Variables|Default|SetIsAlive false)
      (Development|PrintString "Dead"))))

(event Custom|Attack
  (params (ATK :type Float%20%28double-precision%29) (Target :type BP%20Unit%20Component%20Object%20Reference))
  (if (Variables|Default|GetIsAlive)
    (CallFunction|ReceiveDamage Target (Math|Float|Max(Float) (- (Variables|Default|GetATK) (Variables|BP_UnitComponent_C|GetDEF Target)) 1.0))))

(event EventBeginPlay)

(event EventTick
  (params (DeltaSeconds :type Float%20%28single-precision%29)))