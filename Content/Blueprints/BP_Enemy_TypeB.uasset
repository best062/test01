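; Enemy Blueprint that starts a battle when the player stays inside its trigger box through a short delay after a sound cue.
; It saves the player's transform in GI_Mygame, moves both to hardcoded arena spots, switches to BattleCam and opens UI_BattleUI with itself as CurrentEnemy.
; A never-reset DoOnce precedes the player cast, so the first overlap by any actor uses up the trigger.
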(event OnComponentBeginOverlap(box_0)
  (params (OverlappedComponent :type Primitive%20Component%20Object%20Reference) (OtherActor :type Actor%20Object%20Reference) (OtherComp :type Primitive%20Component%20Object%20Reference) (OtherBodyIndex :type Integer) (bFromSweep :type Boolean) (SweepResult :type Hit%20Result%20Structure%20%28by%20ref%29))
  (bind _returnvalue (Game|GetPlayerController 0))
  (Utilities|FlowControl|DoOnce false
    (:Completed
      (bind _asbp_third_person_character (Utilities|Casting|CastToBP_ThirdPersonCharacter OtherActor))
      (Variables|Default|SetbIsPlayerInRange true)
      (Audio|PlaySound2D 0 1.0 1.0 0.0 0 0)
      (Utilities|FlowControl|Delay 1.0)
      (if (Variables|Default|GetbIsPlayerInRange)
        (bind _asgi_mygame (Utilities|Casting|CastToGI_Mygame (Game|GetGameInstance)))
        (Variables|/Game/Blueprints/GI_Mygame.GI_Mygame_C|SetPreBattleTranform _asgi_mygame (Transformation|GetActorTransform _asbp_third_person_character))
        (Transformation|Teleport _asbp_third_person_character "106758.000000,305300.000000,-2409.000000" "0, 0, 0")
        (Transformation|SetActorLocation "105998.000000,305300.000000,-2430.000000" false false)
        (Game|Player|SetViewTargetwithBlend (Game|GetPlayerController 0) (Variables|Default|GetBattleCam) 0.0 "VTBlend_Linear" 0.0 false)
        (Viewport|RemoveAllWidgets)
        (bind _returnvalue_2 (UserInterface|CreateWidget "/Game/UI/UI_BattleUI.UI_BattleUI_C"))
        (UserInterface|Viewport|AddtoViewport _returnvalue_2 0)
        (Variables|/Game/UI/UI_BattleUI.UI_BattleUI_C|SetCurrentEnemy _returnvalue_2 self)
        (Widget|SetKeyboardFocus _returnvalue_2)
        (Input|SetInputModeGameandUI _returnvalue _returnvalue_2 "DoNotLock" true false)
        (Variables|/Script/Engine.PlayerController|SetbShowMouseCursor _returnvalue true)))))

(event OnComponentEndOverlap(box_0)
  (params (OverlappedComponent :type Primitive%20Component%20Object%20Reference) (OtherActor :type Actor%20Object%20Reference) (OtherComp :type Primitive%20Component%20Object%20Reference) (OtherBodyIndex :type Integer))
  (Utilities|Casting|CastToBP_ThirdPersonCharacter OtherActor)
  (Variables|Default|SetbIsPlayerInRange false))

(event EventBeginPlay
  (Variables|Default|Sethome (Transformation|GetActorTransform)))

(event Collision|EventActorBeginOverlap
  (params (OtherActor :type Actor%20Object%20Reference)))

(event EventTick
  (params (DeltaSeconds :type Float%20%28single-precision%29)))

(fn ConstructionScript)